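; Dialogue component that shows and advances a conversation each time Interact is called.
; The first call creates a WB_Dialogue widget with the speaker name and current row's text, while later calls update it.
; Each data table row names the next row and table, chaining lines across tables.
; A row's end flag makes the following call close the widget, leaving that next-row pointer for later conversations.
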(event EventInteract
  (params (playerref :type BP%20First%20Person%20Character%20Object%20Reference))
  (if (Variables|Default|GetEndDialogue)
    (Widget|RemovefromParent (Variables|Default|GetDialogueWidget))
    (Variables|Default|SetEndDialogue false)
    (Variables|Default|SetDialogueWidget 0)
    (else
      (Utilities|IsValid (Variables|Default|GetDialogueWidget)
        (:Is%20Valid
          (bind _returnvalue (Utilities|GetDataTableRow (Variables|Default|GetData%20Table) (Variables|Default|GetRow%20Name))
            (:then
              (Default|UpdateDialogue (Variables|Default|GetDialogueWidget) (.Dialogue (Utilities|Struct|BreakDialogue_Structure _returnvalue)))
              (Variables|Default|SetRow%20Name (.Row (Utilities|Struct|BreakDialogue_Structure _returnvalue)))
              (Variables|Default|SetData%20Table (.DataTable (Utilities|Struct|BreakDialogue_Structure _returnvalue)))
              (Variables|Default|SetEndDialogue (.EndDialogue (Utilities|Struct|BreakDialogue_Structure _returnvalue))))))
        (:Is%20Not%20Valid
          (bind _returnvalue_2 (Utilities|GetDataTableRow (Variables|Default|GetData%20Table) (Variables|Default|GetRow%20Name))
            (:then
              (bind _returnvalue_3 (UserInterface|CreateWidget "/Game/Dialogue2/WB_Dialogue.WB_Dialogue_C" 0 (Utilities|Text|ToText(Name) (Variables|Default|GetName)) (.Dialogue (Utilities|Struct|BreakDialogue_Structure _returnvalue_2))))
              (bind _output_get (Variables|Default|SetDialogueWidget _returnvalue_3))
              (UserInterface|Viewport|AddtoViewport _output_get 0)
              (Variables|Default|SetRow%20Name (.Row (Utilities|Struct|BreakDialogue_Structure _returnvalue_2)))
              (Variables|Default|SetData%20Table (.DataTable (Utilities|Struct|BreakDialogue_Structure _returnvalue_2)))
              (Variables|Default|SetEndDialogue (.EndDialogue (Utilities|Struct|BreakDialogue_Structure _returnvalue_2))))))))))