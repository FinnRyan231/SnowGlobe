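; BP_WindController is an actor that switches wind on and off for materials through Material Parameter Collections.
; Its construction script writes the WindOn state and speed multiplier to MPC_wind.
; ToggleWind flips WindOn and updates intensity in MPC_wind plus WindSpeed in MPC_VegetationMaterialParameters, which construction leaves untouched.
; The event graph holds no active logic.
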(event EventBeginPlay)

(event Collision|EventActorBeginOverlap
  (params (OtherActor :type Actor%20Object%20Reference)))

(event EventTick
  (params (DeltaSeconds :type Float%20%28single-precision%29)))

(fn ConstructionScript
  (Rendering|Material|SetScalarParameterValue "/Game/Objects/PSG_LTX/Material/MPC/MPC_wind.MPC_wind" "wind_intensity" (select (Variables|Default|GetWindOn) 1.0 0.0) :!class /Script/Engine.KismetMaterialLibrary)
  (Rendering|Material|SetScalarParameterValue "/Game/Objects/PSG_LTX/Material/MPC/MPC_wind.MPC_wind" "wind_speed_mult" (Variables|Default|GetWindSpeedMultiplier) :!class /Script/Engine.KismetMaterialLibrary))

(fn ToggleWind
  (Variables|Default|SetWindOn (not (Variables|Default|GetWindOn)))
  (Rendering|Material|SetScalarParameterValue "/Game/Objects/PSG_LTX/Material/MPC/MPC_wind.MPC_wind" "wind_intensity" (select (Variables|Default|GetWindOn) 1.0 0.0) :!class /Script/Engine.KismetMaterialLibrary)
  (Rendering|Material|SetScalarParameterValue "/Game/Objects/PSG_LTX/Material/MPC/MPC_VegetationMaterialParameters.MPC_VegetationMaterialParameters" "WindSpeed" (select (Variables|Default|GetWindOn) 1.0 0.0) :!class /Script/Engine.KismetMaterialLibrary))