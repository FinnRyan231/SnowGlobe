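; BPC_Interact is an actor component for an interaction system, pairing an on-screen interact widget with a proximity trace around its owner.
; On BeginPlay it creates a WBP_Interact widget, stores it and adds it to the viewport.
; Every Tick, InteractionTrace runs a Visibility sphere trace starting and ending at the owner's location.
; The trace result is unused, so nothing yet drives the widget or triggers an interaction.
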(event Custom|CreateInteractDisplay
  ;[0.15 0.15 0.15 0.5] Create interaction display
  (bind _returnvalue (UserInterface|CreateWidget "/Game/InteractUI/WBP_Interact.WBP_Interact_C"))
  (bind _output_get (Variables|Default|SetNewVar _returnvalue))
  (UserInterface|Viewport|AddtoViewport _output_get 0))

(event EventBeginPlay
  (CallFunction|CreateInteractDisplay))

(event EventTick
  (params (DeltaSeconds :type Float%20%28single-precision%29))
  (CallFunction|InteractionTrace))

(fn InteractionTrace
  (bind _returnvalue (Components|GetOwner))
  (bind _returnvalue_2 (Transformation|GetActorLocation _returnvalue))
  (Collision|SphereTraceByChannel _returnvalue_2 _returnvalue_2 0.0 "TraceTypeQuery1" false 0 "None"))