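; BP_Snowglobe is a snowglobe Blueprint that shows a multi-line dialogue on screen, one entry at a time.
; Each call to its custom event increments TalkIndex and writes that Dialogue entry into a DialogueBox widget, created and added to the viewport when none exists.
; Once the entries run out, the event removes the widget, clears the reference and resets the index to -1 so the dialogue can replay.
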(event Custom|CustomEvent
  (Math|Integer|IncrementInt (Variables|Default|GettalkIndex)
    (:%20%20
      (if (< (Variables|Default|GettalkIndex) (Utilities|Array|Length (Variables|Default|GetDialogue)))
        (Variables|Default|GetUI
          (:then
            _)
          (:else
            (bind _returnvalue (UserInterface|CreateWidget "/Game/Dialogue/DialogueBox.DialogueBox_C" (Game|GetPlayerController 0)))
            (bind _output_get (Variables|Default|SetUI _returnvalue))
            (UserInterface|Viewport|AddtoViewport _output_get 0)))
        (Rendering|Components|TextRender|SetText (Variables|/Game/Dialogue/DialogueBox.DialogueBox_C|GetTalkText (Variables|Default|GetUI)) (Utilities|Text|ToText(String) (Utilities|Array|Get(acopy) (Variables|Default|GetDialogue) (Variables|Default|GettalkIndex))))
        (else
          (Widget|RemovefromParent (Variables|Default|GetUI))
          (Variables|Default|SettalkIndex -1)
          (Variables|Default|SetUI 0))))))

(fn ConstructionScript)